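; FPS projectile Blueprint that detonates on a timer, with explosion effect and sound picked by a patch index.
; SetLifeTimerbyDepth schedules Boom after the supplied lifetime.
; When DepthVal is within the threshold, Boom uses GetPatch's result to choose a per-material emitter at the projectile's transform and a pitched 2D sound.
; The actor is destroyed either way; BeginPlay, overlap and Tick are unused.
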(event `self.setLifeTimerByDepth`
  (params (lifeTime :type "Float (single-precision)"))
  (`KismetSystemLibrary.K2_SetTimer` null "Boom" lifeTime))

(event `Boom`
  (if (<= (`self.depthVal`) (`self.depthTheshold`))
    (bind _returnvalue (`self.getPatch`))
    (set `self.soundIdx` _returnvalue)
    (`GameplayStatics.SpawnEmitterAtLocation` (`|GetArrayItem` (`self.effectsByMaterial`) (`self.soundIdx`)) (.location (`self.GetTransform`)) (.rotation (`self.GetTransform`)) (.scale (`self.GetTransform`)))
    (`GameplayStatics.SpawnSound2D` (`|GetArrayItem` (`self.soundsByMaterial`) (`self.soundIdx`)) 1.0 (`self.soundPitchVal`)))
  (`self.K2_DestroyActor`))

(fn `UserConstructionScript`)